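; BP_WeddingFinaleLogic is a trigger actor that stages the wedding finale when the player walks into its box.
; It hides its listed objects at BeginPlay, then on overlap teleports the FPCharacter to a target point and reveals them.
; Disabling player movement and spawning a moving starfish at its target point sit inside the reveal loop, so one starfish spawns per listed object.
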(event OnComponentBeginOverlap(Box)
  (params (OverlappedComponent :type Primitive%20Component%20Object%20Reference) (OtherActor :type Actor%20Object%20Reference) (OtherComp :type Primitive%20Component%20Object%20Reference) (OtherBodyIndex :type Integer) (bFromSweep :type Boolean) (SweepResult :type Hit%20Result%20Structure%20%28by%20ref%29))
  ;[1 1 1] Player teleportation
  (bind _asfpcharacter (Utilities|Casting|CastToFPCharacter OtherActor))
  (bind _output_get (Variables|Default|SetPlayerReference _asfpcharacter))
  (Transformation|SetActorLocation _output_get (Transformation|GetActorLocation (Variables|Default|GetTpTargetPoint)) false false)
  ;[1 1 1] Enabling of objects
  (for _array_element (Variables|Default|GetObjectsToActivate)
    (Rendering|SetActorHiddenInGame _array_element false)
    ;[1 1 1] Disabling player movement
    (Variables|/Game/Blueprints/FPCharacter.FPCharacter_C|SetCanMove (Variables|Default|GetPlayerReference) false)
    ;[1 1 1] Spawning the moving starfish
    (Game|SpawnActorfromClass "/Game/Blueprints/Blueprint_CP_MovingStarfish.Blueprint_CP_MovingStarfish_C" (Transformation|GetActorTransform (Variables|Default|GetStarfishTargetPoint)) "Undefined" 0 0)))

(event EventBeginPlay
  (for _array_element (Variables|Default|GetObjectsToActivate)
    (Rendering|SetActorHiddenInGame _array_element true)))

(fn ConstructionScript)