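; First-person character Blueprint that handles walking, running and mouse-style look from player input.
; Axis inputs move along the yaw-only control rotation and turn the controller, with look values clamped and scaled by a sensitivity.
; Left Shift held sets a running flag, which Tick uses to pick the current speed.
; That speed scales the movement input vector; the movement component's max speed is never set.
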(event EventTick
  (params (DeltaSeconds :type Float%20%28single-precision%29))
  ;[1 1 1] RunningSpeedManagement
  (if (Variables|Default|GetIsRunning)
    (Variables|Default|SetCurrentMovementSpeed (Variables|Default|GetRunningSpeedValue))
    (else
      (Variables|Default|SetCurrentMovementSpeed (Variables|Default|GetWalkingSpeedValue)))))

(event Input|AxisEvents|InputAxisForward/Backward
  (params (AxisValue :type Float%20%28single-precision%29))
  ;[1 1 1] Movement
  (Pawn|Input|AddMovementInput (* (Math|Vector|GetForwardVector (Math|Rotator|MakeRotator 0.0 0.0 (.Yaw (Math|Rotator|BreakRotator (Pawn|GetControlRotation :!class /Script/Engine.Pawn))))) (Variables|Default|GetCurrentMovementSpeed)) AxisValue false))

(event Input|AxisEvents|InputAxisLeft/Right
  (params (AxisValue :type Float%20%28single-precision%29))
  ;[1 1 1] Movement
  (Pawn|Input|AddMovementInput (* (Variables|Default|GetCurrentMovementSpeed) (Math|Vector|GetRightVector (Math|Rotator|MakeRotator 0.0 0.0 (.Yaw (Math|Rotator|BreakRotator (Pawn|GetControlRotation :!class /Script/Engine.Pawn)))))) AxisValue false))

(event Input|AxisEvents|InputAxisLoopUp/LookDown
  (params (AxisValue :type Float%20%28single-precision%29))
  ;[1 1 1] Rotation
  (Pawn|Input|AddControllerPitchInput (* (Math|Float|Clamp(Float) AxisValue -1.0) (Variables|Default|GetRotationSensitivity))))

(event Input|AxisEvents|InputAxisLookLeft/LookRight
  (params (AxisValue :type Float%20%28single-precision%29))
  ;[1 1 1] Rotation
  (Pawn|Input|AddControllerYawInput (* (Variables|Default|GetRotationSensitivity) (Math|Float|Clamp(Float) AxisValue -1.0))))

(event Input|KeyboardEvents|LeftShift
  (params (Key :type Key%20Structure :default "None"))
  ;[1 1 1] RunningSpeedManagement
  (:Pressed
    (Variables|Default|SetIsRunning true))
  (:Released
    (Variables|Default|SetIsRunning false)))

(fn ConstructionScript)